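; Functional test checking that ammo pickups stop being consumed once the player's weapon reserves are full.
; PrepareTest works out how many pickups fill the reserves from the weapon's ammo values, then spawns copies on the placed pickup, leaving one surplus.
; StartTest destroys the platform under the player, waits for the fall, and passes only if exactly one pickup remains active.
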(event EventPrepareTest
  (bind _pickupammo (Variables|Default|GetPickupAmmo))
  (bind _playerpawn (Variables|Default|GetPlayerPawn)
    (:then
      (Utilities|IsValid (Class|ShooterCharacter|GetWeapon _playerpawn)
        (:Is%20Valid
          (bind _output_get (Variables|Default|SetPlayerWeapon (Class|ShooterCharacter|GetWeapon _playerpawn)))
          ;[1 1 1] Calculate amount of pickups needed to fill entire reserves for player
          (bind _output_get_2 (Variables|Default|SetAmmoPickupsToMax (Math|Float|Ceil (/ (/ (Math|Conversions|ToFloat(Integer) (- (Class|ShooterWeapon|GetMaxAmmo _output_get) (Class|ShooterWeapon|GetCurrentAmmo _output_get))) (Math|Conversions|ToFloat(Integer) (Class|ShooterWeapon|GetAmmoPerClip _output_get))) (Math|Conversions|ToFloat(Integer) (Variables|/Script/ShooterGame.ShooterPickup_Ammo|GetAmmoClips (Variables|Default|GetPickupAmmo)))))))
          ;[1 1 1] Spawn ammo pickups, enough so one will be left over after picked up all
          (Utilities|Array|Add (Variables|Default|GetPickups) (Variables|Default|GetPickupAmmo))
          (for _index (range 0 (- _output_get_2 1))
            (bind _returnvalue (Game|SpawnActorfromClass (Utilities|GetClass _pickupammo) (Transformation|GetActorTransform _pickupammo) "AlwaysSpawn" 0 0))
            (Utilities|Array|Add (Variables|Default|GetPickups) _returnvalue)))
        (:Is%20Not%20Valid
          (Class|FunctionalTest|FinishTest "Failed" "Player weapon invalid"))))
    (:else
      (Class|FunctionalTest|FinishTest "Failed" "Unassigned reference"))))

(event EventStartTest
  (Actor|DestroyActor (Variables|Default|GetPlayerPlatform))
  (Utilities|FlowControl|Delay (Variables|Default|GetFall%20Delay))
  (Variables|Default|SetActivePickups 0)
  ;[1 1 1] Count remaining pickups after player has fallen onto them
  (for _array_element (Variables|Default|GetPickups)
    (if (Variables|/Script/ShooterGame.ShooterPickup|GetbIsActive _array_element)
      (Math|Integer|IncrementInt (Variables|Default|GetActivePickups))))
  (if (== (Variables|Default|GetActivePickups) 1)
    (Class|FunctionalTest|FinishTest "Succeeded" "Test OK")
    (else
      (Class|FunctionalTest|FinishTest "Failed" (Utilities|String|Append (Utilities|String|MakeLiteralString "Wrong amount of pickups left. Expected 1 values was : ") (Utilities|String|ToString(Integer) (Variables|Default|GetActivePickups)))))))

(fn ConstructionScript)