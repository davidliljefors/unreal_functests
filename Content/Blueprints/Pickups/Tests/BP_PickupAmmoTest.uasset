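; Functional test that checks an ammo pickup grants the correct ammo to a player pawn's ShooterWeapon_Instant.
; PrepareTest computes expected ammo from the weapon's current ammo, clip size and the pickup's clip count, failing on missing references or wrong weapon.
; StartTest destroys the player platform to set the test in motion.
; Tick succeeds once ammo exactly matches the expected value, with no failure branch for mismatches.
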(event EventPrepareTest
  (Development|PrintString "start 2")
  (bind _playerpawn (Variables|Default|GetPlayerPawn)
    (:then
      (bind _asshooter_weapon_instant (Utilities|Casting|CastToShooterWeapon_Instant (Class|ShooterCharacter|GetWeapon _playerpawn))
        (:then
          (bind _output_get (Variables|Default|SetPlayerWeapon _asshooter_weapon_instant))
          (Variables|Default|SetStartingAmmo (Class|ShooterWeapon|GetCurrentAmmo _output_get))
          (bind _pickupammo (Variables|Default|GetPickupAmmo)
            (:then
              (Variables|Default|SetExpectedAmmo (+ (Class|ShooterWeapon|GetCurrentAmmo (Variables|Default|GetPlayerWeapon)) (* (Class|ShooterWeapon|GetAmmoPerClip (Variables|Default|GetPlayerWeapon)) (Variables|/Script/ShooterGame.ShooterPickup_Ammo|GetAmmoClips _pickupammo)))))
            (:else
              (Class|FunctionalTest|FinishTest "Failed" "Pickup not Assigned"))))
        (:CastFailed
          (Class|FunctionalTest|FinishTest "Failed" "PlayerPawn carrying wrong weapon"))))
    (:else
      (Class|FunctionalTest|FinishTest "Failed" "No PlayerPawn Assigned"))))

(event EventStartTest
  (bind _playerplatform (Variables|Default|GetPlayerPlatform)
    (:then
      (Actor|DestroyActor _playerplatform))
    (:else
      (Class|FunctionalTest|FinishTest "Failed" "PlayerPlatform not assigned"))))

(event EventTick
  (params (DeltaSeconds :type Float%20%28single-precision%29))
  (if (== (Class|ShooterWeapon|GetCurrentAmmo (Variables|Default|GetPlayerWeapon)) (Variables|Default|GetExpectedAmmo))
    (Class|FunctionalTest|FinishTest "Succeeded" "Ammo after pickup was correct")))

(fn ConstructionScript)