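; BP_PickupAmmoIsForWeaponTest is a functional test checking that an ammo pickup only reports it can be picked up by a suitable pawn.
; On start it requires an assigned PlayerPawn carrying a ShooterWeapon_Instant, failing otherwise.
; It then expects CanBePickedUp to return false with no pawn and true for the player, finishing the test with a matching result message.
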(event EventPrepareTest)

(event EventStartTest
  (bind _playerpawn (Variables|Default|GetPlayerPawn)
    (:then
      (Utilities|Casting|CastToShooterWeapon_Instant (Class|ShooterCharacter|GetWeapon _playerpawn)
        (:then
          (if (Class|ShooterPickupAmmo|CanbePickedUp (Variables|Default|GetPickupAmmo))
            (Class|FunctionalTest|FinishTest "Failed" "CanBePickedUp on null was true, expected : false")
            (elif (Class|ShooterPickupAmmo|CanbePickedUp (Variables|Default|GetPickupAmmo) (Variables|Default|GetPlayerPawn))
              (Class|FunctionalTest|FinishTest "Succeeded" "Test OK")
              (else
                (Class|FunctionalTest|FinishTest "Failed" "CanBePickedUp on player was false, expected : true")))))
        (:CastFailed
          (Class|FunctionalTest|FinishTest "Failed" "Testing PlayerPawn carrying wrong weapon"))))
    (:else
      (Class|FunctionalTest|FinishTest "Failed" "No PlayerPawn Assigned"))))

(event EventTick
  (params (DeltaSeconds :type Float%20%28single-precision%29)))

(fn ConstructionScript)