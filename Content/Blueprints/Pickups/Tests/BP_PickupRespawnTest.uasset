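; Functional test that checks an ammo pickup becomes active again after its respawn time.
; PrepareTest validates the assigned pickup, player and platform, then destroys the platform, waits for a fall time, and destroys the character.
; StartTest waits the pickup's respawn time scaled by a multiplier, then passes only if the pickup is active.
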(event EventPrepareTest
  (bind _pickupammo (Variables|Default|GetPickupAmmo)
    (:then
      (if (Variables|/Script/ShooterGame.ShooterPickup|GetbIsActive _pickupammo)
        (Variables|Default|GetPlayerCharacter
          (:then
            (bind _playerplatform (Variables|Default|GetPlayerPlatform)
              (:then
                (Actor|DestroyActor _playerplatform)
                (Utilities|FlowControl|Delay (Variables|Default|GetFallTime))
                (Actor|DestroyActor (Variables|Default|GetPlayerCharacter)))
              (:else
                (Class|FunctionalTest|FinishTest "Failed" "PlayerPlatform not assigned"))))
          (:else
            (Class|FunctionalTest|FinishTest "Failed" "PlayerCharacter not assigned")))
        (else
          (Class|FunctionalTest|FinishTest "Failed" "Pickup not active on start"))))
    (:else
      (Class|FunctionalTest|FinishTest "Failed" "Pickup not assigned"))))

(event EventStartTest
  (Utilities|FlowControl|Delay (* (Variables|/Script/ShooterGame.ShooterPickup|GetRespawnTime (Variables|Default|GetPickupAmmo)) (Variables|Default|GetWaitTimeMultiplier)))
  (if (Variables|/Script/ShooterGame.ShooterPickup|GetbIsActive (Variables|Default|GetPickupAmmo))
    (Class|FunctionalTest|FinishTest "Succeeded" "Test OK")
    (else
      (Class|FunctionalTest|FinishTest "Failed" "Pickup was not respawned after set time"))))

(fn ConstructionScript)